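; Render-tools actor that applies rendering console variables when play begins.
; SetupCVars calls four setup functions, each gated by an Enable flag: sky atmosphere quality, camera cut translation threshold, volumetric render target mode and upsampling, and raytracing shadows.
; The raytracing step disables two-sided geometry shadows to fix wrong shadows with Nanite.
; A few alternative commands sit unconnected and never run.
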(event `self.ReceiveBeginPlay`
  (`self.SetupCVars`))

(fn `CameraCutTranslationSetup`
  ;[1 1 1] Usefull with skyatmosphere
  (`KismetSystemLibrary.ExecuteConsoleCommand` "r.CameraCutTranslationThreshold 1000000" null))

(fn `RaytracingSetup`
  ;[1 1 1] Fix wrong shadows on geometry with nanite & require all geometry to be 2sided to have shadows
  (`KismetSystemLibrary.ExecuteConsoleCommand` "r.RayTracing.Shadows.EnableTwoSidedGeometry 0" null))

(fn `SetupCVars`
  (if (`self.EnableSkyAtmosphereSetup`)
    (`self.SkyAtmosphereSetup`))
  (if (`self.EnableCameraCutTranslationSetup`)
    (`self.CameraCutTranslationSetup`))
  (if (`self.EnableVolumetricSetup`)
    (`self.VolumetricSetup`))
  (if (`self.EnableRaytracingSetup`)
    (`self.RaytracingSetup`)))

(fn `SkyAtmosphereSetup`
  (`KismetSystemLibrary.ExecuteConsoleCommand` "r.SkyAtmosphere.SampleCountMax 64" null)
  (`KismetSystemLibrary.ExecuteConsoleCommand` "r.SkyAtmosphere.FastSkyLUT 0" null)
  (`KismetSystemLibrary.ExecuteConsoleCommand` "r.SkyAtmosphere.AerialPerspectiveLUT.FastApplyOnOpaque 0" null)
  (`KismetSystemLibrary.ExecuteConsoleCommand` "r.SkyAtmosphere.AerialPerspectiveLUT.Depth 96" null)
  (`KismetSystemLibrary.ExecuteConsoleCommand` "r.SkyAtmosphere.MultiScatteringLUT.HighQuality 1" null))

(fn `UserConstructionScript`)

(fn `VolumetricSetup`
  (`KismetSystemLibrary.ExecuteConsoleCommand` "r.VolumetricRenderTarget 1" null)
  (`KismetSystemLibrary.ExecuteConsoleCommand` "r.VolumetricRenderTarget.Mode 1" null)
  (`KismetSystemLibrary.ExecuteConsoleCommand` "r.VolumetricRenderTarget.UpsamplingMode 4" null))